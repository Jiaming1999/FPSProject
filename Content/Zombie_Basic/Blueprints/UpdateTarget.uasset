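; Behavior Tree service for the zombie AI that updates its target from the first player's proximity.
; Each tick it compares squared pawn-to-player distance against the squared PerceptionDistance, using no line-of-sight check.
; In range, it writes the player to the AITarget blackboard key and switches AIState to the second zombie state.
; Otherwise it clears the target and sets AIState back to the first state.
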(event `self.ReceiveTickAI`
  (params (OwnerController :type "AIController Object Reference") (ControlledPawn :type "Pawn Object Reference") (DeltaSeconds :type "Float (single-precision)"))
  (bind _returnvalue (`GameplayStatics.GetPlayerCharacter` 0))
  (if (< (`KismetMathLibrary.Vector_DistanceSquared` (`Actor.K2_GetActorLocation` ControlledPawn) (`Actor.K2_GetActorLocation` _returnvalue)) (`KismetMathLibrary.Square` (`self.PerceptionDistance`)))
    (`BTFunctionLibrary.SetBlackboardValueAsObject` (`self.AITarget`) _returnvalue)
    (`BTFunctionLibrary.SetBlackboardValueAsEnum` (`self.AIState`) (enumliteral `/Game/Zombie_Basic/Blueprints/Zombie_AISTATE` "NewEnumerator1"))
    (else
      (`BTFunctionLibrary.SetBlackboardValueAsObject` (`self.AITarget`))
      (`BTFunctionLibrary.SetBlackboardValueAsEnum` (`self.AIState`) (enumliteral `/Game/Zombie_Basic/Blueprints/Zombie_AISTATE` "NewEnumerator0")))))