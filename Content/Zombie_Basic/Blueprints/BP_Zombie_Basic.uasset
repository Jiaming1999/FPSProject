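; BP_Zombie_Basic is a basic zombie enemy that takes damage from shots and dies.
; Capsule overlaps with FirstPersonProjectile or BP_Bullet call ApplyDamage, which subtracts random damage and sets IsDead when its check reaches zero.
; The death check and the subtraction use separate random rolls.
; Kill stops the AI brain, switches the mesh to ragdoll physics, disables capsule collision and destroys the actor after a delay.
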(event `self.CapsuleComponent.OnComponentBeginOverlap`
  (params (OverlappedComponent :type "PrimitiveComponent Object Reference") (OtherActor :type "Actor Object Reference") (OtherComp :type "PrimitiveComponent Object Reference") (OtherBodyIndex :type Integer) (bFromSweep :type Boolean) (SweepResult :type "HitResult Structure (by ref)"))
  (cast `/Game/FirstPersonBP/Blueprints/FirstPersonProjectile` OtherActor
    (:`then`
      _)
    (:`CastFailed`
      (cast `/Game/BP/Actor/Weapon/BP_Bullet` OtherActor)))
  (`self.Apply Damage`)
  (if (`self.IsDead`)
    (`self.Kill`)))

(event `Kill`
  (bind _mesh (`self.Mesh`))
  (`BrainComponent.StopLogic` (`AIController.BrainComponent` (`AIBlueprintHelperLibrary.GetAIController` self)) "")
  (`PrimitiveComponent.SetCollisionProfileName` _mesh "Ragdoll" true)
  (`PrimitiveComponent.SetSimulatePhysics` _mesh true)
  (`PrimitiveComponent.SetCollisionProfileName` (`self.CapsuleComponent`) "NoCollision" true)
  (`KismetSystemLibrary.Delay` 5.0)
  (`self.K2_DestroyActor`))

(fn `Apply Damage`
  (bind _returnvalue (- (`self.Health`) (`KismetMathLibrary.RandomFloatInRange` 30.0 70.0)))
  (if (<= _returnvalue 0.0)
    (set `self.Health` 0.0)
    (set `self.IsDead` true)
    (else
      (set `self.Health` _returnvalue))))

(fn `UserConstructionScript`)