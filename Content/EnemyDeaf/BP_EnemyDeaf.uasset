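; BP_EnemyDeaf is an enemy character that chases the player based on how loud they are and how close they are.
; Each Tick it divides the FirstPersonCharacter's Decibel value by the distance to the player, prints the ratio and starts ChasePlayer at a fixed threshold.
; ChasePlayer uses AI MoveTo toward the player and calls itself again one second after each success, without rechecking loudness.
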(event `self.ReceiveBeginPlay`
  (set `CharacterMovementComponent.MaxWalkSpeed` 400.0 (`self.CharacterMovement`)))

(event `self.ReceiveTick`
  (params (DeltaSeconds :type "Float (single-precision)"))
  (bind _returnvalue (`GameplayStatics.GetPlayerCharacter` 0))
  ;[1 1 1] calculate whether to chase player based on player decibels and distance to player
  (bind _asfirst_person_character (cast `/Game/FirstPersonBP/Blueprints/FirstPersonCharacter` _returnvalue))
  (bind _returnvalue_2 (/ (`/Game/FirstPersonBP/Blueprints/FirstPersonCharacter.Decibel` _asfirst_person_character) (`KismetMathLibrary.Vector_Distance` (`self.K2_GetActorLocation` _returnvalue) (`self.K2_GetActorLocation`))))
  (`KismetSystemLibrary.PrintString` (`KismetStringLibrary.Conv_DoubleToString` _returnvalue_2))
  (if (>= _returnvalue_2 0.03)
    (`self.ChasePlayer`)))

(event `ChasePlayer`
  ;[1 1 1] chase player
  (`|AIMoveTo` self (0.0 0.0 0.0) (`GameplayStatics.GetPlayerCharacter` 0)
    (:`OnSuccess`
      (`KismetSystemLibrary.Delay` 1.0)
      (`self.ChasePlayer`))))

(fn `UserConstructionScript`)