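; BP_EnemyBlind is an enemy character that chases the player using AI movement.
; BeginPlay sets its walk speed, and Tick starts a chase when its AI controller has line of sight to the player within a very short distance.
; ChasePlayer runs AI MoveTo on the player and calls itself again after a short delay on each success, with no handling for failed moves.
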(event `self.ReceiveBeginPlay`
  (set `CharacterMovementComponent.MaxWalkSpeed` 400.0 (`self.CharacterMovement`)))

(event `self.ReceiveTick`
  (params (DeltaSeconds :type "Float (single-precision)"))
  ;[1 1 1] check for line of sight in order to chase player
  (if (`Controller.LineOfSightTo` (`AIBlueprintHelperLibrary.GetAIController` self) (`GameplayStatics.GetPlayerCharacter` 0) (`self.GetActorEyesViewPoint`) false)
    (if (<= (`KismetMathLibrary.Vector_Distance` (`self.K2_GetActorLocation` (`GameplayStatics.GetPlayerCharacter` 0)) (`self.K2_GetActorLocation`)) 10.0)
      (`self.ChasePlayer`))))

(event `ChasePlayer`
  ;[1 1 1] chase player
  (`|AIMoveTo` self (0.0 0.0 0.0) (`GameplayStatics.GetPlayerCharacter` 0)
    (:`OnSuccess`
      (`KismetSystemLibrary.Delay` 1.0)
      (`self.ChasePlayer`))))

(fn `UserConstructionScript`)