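; Small 7.62 ammo box prop that assembles its cartridges in the construction script, with no active runtime logic.
; Three staggered rows of instanced meshes, with the middle row flipped, fill the box.
; A scaled CountAmmoIn value then sets how many instances are removed, either from the first index or at random through a seeded stream.
; Options control cap and ammo visibility, ammo shadows, and separate cull distances for box and ammo.
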(fn `UserConstructionScript`
  (bind _ammo_visible (`self.Ammo visible`))
  (`|ExecutionSequence`
    (:`then_0`
      ;[1 1 1] Cap Visible
      (`/Game/Collectibles/Ammo_and_bullets_Pack/Blueprints/Macroses/On-Off_Macro.On/Off Macro` (`self.StaticMeshComponent0`) (`self.Visible Box`)))
    (:`then_1`
      ;[1 1 1] First row
      (for _index (range 10)
        (`InstancedStaticMeshComponent.AddInstance` (`self.InstancedStaticMesh`) (`KismetMathLibrary.MakeTransform` (`KismetMathLibrary.MakeVector` (* _index (`self.Space`))) (struct :`Pitch` 90.0) (1.0 1.0 1.0)))))
    (:`then_2`
      ;[1 1 1] Second row
      (for _index_2 (range 9)
        (`InstancedStaticMeshComponent.AddInstance` (`self.InstancedStaticMesh`) (`KismetMathLibrary.MakeTransform` (`KismetMathLibrary.MakeVector` (+ (* _index_2 (`self.Space`)) 0.5) 1.1 7.1) (struct :`Pitch` -90.0)))))
    (:`then_3`
      ;[1 1 1] Third row
      (for _index_3 (range 10)
        (`InstancedStaticMeshComponent.AddInstance` (`self.InstancedStaticMesh`) (`KismetMathLibrary.MakeTransform` (`KismetMathLibrary.MakeVector` (* _index_3 (`self.Space`)) 2.2) (struct :`Pitch` 90.0)))))
    (:`then_4`
      ;[1 1 1] Set up seed for random seed
      (set `self.Count ammo seed` (`KismetMathLibrary.MakeRandomStream` (`self.= Count ammo seed =`))))
    (:`then_5`
      ;[1 1 1] Amount of remote ammo
      (if (`self.Use random count of ammo`)
        (for _ (range (+ (`KismetMathLibrary.FTrunc` (* (`self.Count ammo in %`) 0.29)) 1))
          (`InstancedStaticMeshComponent.RemoveInstance` (`self.InstancedStaticMesh`) (`KismetMathLibrary.RandomIntegerInRangeFromStream` 0 (`InstancedStaticMeshComponent.GetInstanceCount` (`self.InstancedStaticMesh`)) (`self.Count ammo seed`))))
        (else
          (for _ (range (`KismetMathLibrary.FTrunc` (`KismetMathLibrary.Abs` (* (`self.Count ammo in %`) 0.29))))
            (`InstancedStaticMeshComponent.RemoveInstance` (`self.InstancedStaticMesh`) 0)))))
    (:`then_6`
      ;[1 1 1] Ammo Visible
      (`SceneComponent.SetVisibility` (`self.InstancedStaticMesh`) _ammo_visible false)
      (`PrimitiveComponent.SetCastShadow` (`self.InstancedStaticMesh`) _ammo_visible))
    (:`then_7`
      ;[1 1 1] Draw Distance
      (`PrimitiveComponent.SetCullDistance` (`self.InstancedStaticMesh`) (`self.Ammo Draw Distance (0 - Infinity)`))
      (`PrimitiveComponent.SetCullDistance` (`self.StaticMeshComponent01`) (`self.Box Draw Distance (0 - Infinity)`))
      (`PrimitiveComponent.SetCullDistance` (`self.StaticMeshComponent0`) (`self.Box Draw Distance (0 - Infinity)`)))))