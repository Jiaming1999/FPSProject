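; BP_300GaSmallBox is a small ammo box prop with no active runtime logic.
; Its Construction Script toggles visibility and shadow casting on the instanced ammo mesh and picks one of two box materials.
; It also sets separate cull distances for the box and its ammo, so each can have its own draw range.
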(fn `UserConstructionScript`
  (bind _ammo_visible (`self.Ammo visible`))
  (`|ExecutionSequence`
    (:`then_0`
      ;[1 1 1] Ammo Visible
      (`SceneComponent.SetVisibility` (`self.InstancedStaticMesh`) _ammo_visible false)
      (`PrimitiveComponent.SetCastShadow` (`self.InstancedStaticMesh`) _ammo_visible))
    (:`then_1`
      ;[1 1 1] Material Variant
      (switch `int` (`self.Material variant`)
        (:`1`
          (`PrimitiveComponent.SetMaterial` (`self.StaticMeshComponent0`) 0 "/Game/Collectibles/Ammo_and_bullets_Pack/Materials/Instances/MI_300GaSmallBox.MI_300GaSmallBox"))
        (:`2`
          (`PrimitiveComponent.SetMaterial` (`self.StaticMeshComponent0`) 0 "/Game/Collectibles/Ammo_and_bullets_Pack/Materials/Instances/MI_300GaSmallBoxV2.MI_300GaSmallBoxV2"))))
    (:`then_2`
      ;[1 1 1] Draw Distance
      (`PrimitiveComponent.SetCullDistance` (`self.InstancedStaticMesh`) (`self.Ammo Draw Distance (0 - Infinity)`))
      (`PrimitiveComponent.SetCullDistance` (`self.StaticMeshComponent0`) (`self.Box Draw Distance (0 - Infinity)`)))))